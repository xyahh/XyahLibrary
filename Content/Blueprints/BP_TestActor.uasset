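; BP_TestActor is a scratch test actor holding sample nodes from the Xyah array, utility and actor Blueprint libraries.
; The library calls sit unconnected in the event graph, with BeginPlay and the construction script empty, so none of them run.
; Sorter, ActorSorter, ActorRemoveIf and ActorFindIf are sample predicates comparing values or actor name lengths, shaped for the name-based array functions, whose predicate names are left unset.
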(event `self.ReceiveBeginPlay`)

(fn `Actor FindIf`
  (params (NamedActor :type "/Game/Blueprints/BP_NamedActor Object Reference"))
  (returns (RetVal :type Boolean))
  (return (>= (`KismetStringLibrary.Len` (`/Game/Blueprints/BP_NamedActor.Name` NamedActor)) 3)))

(fn `Actor RemoveIf`
  (params (A :type "/Game/Blueprints/BP_NamedActor Object Reference"))
  (returns (Return :type Boolean))
  (return (< (`KismetStringLibrary.Len` (`/Game/Blueprints/BP_NamedActor.Name` A)) 6)))

(fn `Actor Sorter`
  (params (A :type "/Game/Blueprints/BP_NamedActor Object Reference") (B :type "/Game/Blueprints/BP_NamedActor Object Reference"))
  (returns (RetVal :type Boolean))
  (return (< (`KismetStringLibrary.Len` (`/Game/Blueprints/BP_NamedActor.Name` A)) (`KismetStringLibrary.Len` (`/Game/Blueprints/BP_NamedActor.Name` B)))))

(fn `Sorter`
  (params (A :type Integer) (B :type Integer))
  (returns (Return :type Boolean))
  (return (< A B)))

(fn `UserConstructionScript`)